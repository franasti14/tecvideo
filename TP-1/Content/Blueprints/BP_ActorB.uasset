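; BP_ActorB is an actor that reports its stats and moves and spins continuously.
; On BeginPlay it prints its name, health, resistance, damage, critical damage, speed and rotation speed as one concatenated string, plus a hello message.
; Each Tick applies the velocity and rotation variables as local offsets, with sweep on the movement and no delta-time scaling, so motion depends on frame rate.
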(event `self.ReceiveBeginPlay`
  (`KismetSystemLibrary.PrintString` (`KismetStringLibrary.Concat_StrStr` (`self.Nombre`) (`KismetStringLibrary.Conv_DoubleToString` (`self.Vida`)) (`KismetStringLibrary.Conv_DoubleToString` (`self.Resistencia`)) (`KismetStringLibrary.Conv_Int64ToString` (`self.Daño`)) (`KismetStringLibrary.Conv_DoubleToString` (`self.Daño Critico`)) (`KismetStringLibrary.Conv_VectorToString` (`self.Velocidad`)) (`KismetStringLibrary.Conv_RotatorToString` (`self.Velrotacion`))) true false)
  (`KismetSystemLibrary.PrintText` "Hello"))

(event `self.ReceiveTick`
  (params (DeltaSeconds :type "Float (single-precision)"))
  (`self.K2_AddActorLocalOffset` (`self.Velocidad`) true)
  (`self.K2_AddActorLocalRotation` (`self.velrotacion`)))

(fn `UserConstructionScript`)