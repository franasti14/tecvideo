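; BP_ActorA is an actor that holds character-style stats (name, health, resistance, damage, critical damage) under Spanish variable names and moves continuously.
; BeginPlay prints those stats, along with its velocity and rotation speed, as one on-screen debug string.
; Tick adds the velocity and rotation variables as local offset and rotation each frame, without delta-time scaling or sweep.
; The damage and health stats are only printed, never applied.
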(event `self.ReceiveBeginPlay`
  (`KismetSystemLibrary.PrintString` (`KismetStringLibrary.Concat_StrStr` (`self.Nombre`) (`KismetStringLibrary.Conv_DoubleToString` (`self.Vida`)) (`KismetStringLibrary.Conv_DoubleToString` (`self.Resistencia`)) (`KismetStringLibrary.Conv_Int64ToString` (`self.Daño`)) (`KismetStringLibrary.Conv_DoubleToString` (`self.Daño Critico`)) (`KismetStringLibrary.Conv_VectorToString` (`self.Velocidad`)) (`KismetStringLibrary.Conv_RotatorToString` (`self.Velrotacion`))) true true (struct :`G` 1.0 :`B` 0.063367 :`A` 1.0) 5.0))

(event `self.ReceiveTick`
  (params (DeltaSeconds :type "Float (single-precision)"))
  (`self.K2_AddActorLocalOffset` (`self.Velocidad`))
  (`self.K2_AddActorLocalRotation` (`self.Velrotacion`)))

(fn `UserConstructionScript`)