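; BP_ActorC is an actor that carries stat variables such as name, health, resistance and damage, and moves and spins continuously.
; BeginPlay prints those stats and both speed variables as one red string, plus a "Vida:" label.
; Tick applies Velocidad as both a swept local offset and an unswept world offset, and adds Velrotacion as world rotation, without delta-time scaling.
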(event `self.ReceiveBeginPlay`
  (`KismetSystemLibrary.PrintString` (`KismetStringLibrary.Concat_StrStr` (`self.Nombre`) (`KismetStringLibrary.Conv_DoubleToString` (`self.Vida`)) (`KismetStringLibrary.Conv_DoubleToString` (`self.Resistencia `)) (`KismetStringLibrary.Conv_Int64ToString` (`self.Daño`)) (`KismetStringLibrary.Conv_DoubleToString` (`self.Daño Critico`)) (`KismetStringLibrary.Conv_RotatorToString` (`self.Velrotacion`)) (`KismetStringLibrary.Conv_VectorToString` (`self.Velocidad`))) true true (struct :`R` 1.0 :`G` 0.050181 :`B` 0.020335 :`A` 1.0))
  (`KismetSystemLibrary.PrintText` "Vida:"))

(event `self.ReceiveTick`
  (params (DeltaSeconds :type "Float (single-precision)"))
  (`self.K2_AddActorLocalOffset` (`self.Velocidad`) true)
  (`self.K2_AddActorWorldRotation` (`self.Velrotacion`))
  (`self.K2_AddActorWorldOffset` (`self.Velocidad`)))

(fn `UserConstructionScript`)